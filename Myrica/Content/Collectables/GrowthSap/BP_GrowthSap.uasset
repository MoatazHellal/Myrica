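; BP_GrowthSap is a collectable that slightly refills the energy bar when a BP_Fey overlaps it.
; On overlap it checks for that exact class, then spawns a scaled-down NS_Curse_Blink Niagara effect at its location.
; It reaches the EnergyBarWidget through BP_Gamemode, adds a small fixed increment to the progress bar's current percent, then destroys itself.
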(event `self.ReceiveActorBeginOverlap`
  (params (OtherActor :type "Actor Object Reference"))
  (if (== (`GameplayStatics.GetObjectClass` OtherActor) "/Game/Fey/BP_Fey.BP_Fey_C")
    (`NiagaraFunctionLibrary.SpawnSystemAtLocation` "/Game/BlinkAndDashVFX/VFX_Niagara/NS_Curse_Blink.NS_Curse_Blink" (`self.K2_GetActorLocation`) (struct) (0.02 0.02 0.02))
    (bind _asbp_gamemode (cast `/Game/Game/Blueprints/BP_Gamemode` (`GameplayStatics.GetGameMode`)))
    (bind _energybarwidget (`/Game/Game/Blueprints/BP_Gamemode.EnergyBarWidget` _asbp_gamemode))
    (bind _percent (`/Game/Widgets/WBP_EnergyBar.GetProgressBarPercent` _energybarwidget))
    (`/Game/Widgets/WBP_EnergyBar.UpdateProgressBar` _energybarwidget (+ _percent 0.01))
    (`self.K2_DestroyActor`)))

(fn `UserConstructionScript`)