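; BP_RunicSwitch is a runic switch that plays the GateActivation level sequence when activated by the player in range.
; Its capsule shows a text prompt when BP_Fey enters and hides it when any overlap ends.
; Activate checks that the player overlaps the capsule, recolors the LightBall red through a dynamic rune material instance, then starts the sequence after a short delay.
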(event `/Game/Game/BPI_Mechanism.Activate`
  (if (`PrimitiveComponent.IsOverlappingActor` (`self.Capsule`) (`GameplayStatics.GetPlayerCharacter` 0))
    (bind _returnvalue (`PrimitiveComponent.CreateDynamicMaterialInstance` (`self.LightBall`) 0 "/Game/Isometric_World/Sky_Temple/Materials/Runes/MI_Temple_Runes_Emissive_01.MI_Temple_Runes_Emissive_01" "None"))
    (`MaterialInstanceDynamic.SetVectorParameterValue` _returnvalue "BaseColor" (struct :`R` 1.0 :`B` 0.031044 :`A` 1.0))
    (`KismetSystemLibrary.Delay` 0.5)
    (bind (_outactor _returnvalue_2) (`LevelSequencePlayer.CreateLevelSequencePlayer` "/Game/Game/Cinematics/GateActivation.GateActivation"))
    (`MovieSceneSequencePlayer.Play` _returnvalue_2)))

(event `self.Capsule.OnComponentBeginOverlap`
  (params (OverlappedComponent :type "PrimitiveComponent Object Reference") (OtherActor :type "Actor Object Reference") (OtherComp :type "PrimitiveComponent Object Reference") (OtherBodyIndex :type Integer) (bFromSweep :type Boolean) (SweepResult :type "HitResult Structure (by ref)"))
  (if (== (`GameplayStatics.GetObjectClass` OtherActor) "/Game/Fey/BP_Fey.BP_Fey_C")
    (`SceneComponent.SetVisibility` (`self.TextRender`) true false)))

(event `self.Capsule.OnComponentEndOverlap`
  (params (OverlappedComponent :type "PrimitiveComponent Object Reference") (OtherActor :type "Actor Object Reference") (OtherComp :type "PrimitiveComponent Object Reference") (OtherBodyIndex :type Integer))
  (`SceneComponent.SetVisibility` (`self.TextRender`) false false))

(fn `UserConstructionScript`)