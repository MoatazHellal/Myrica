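; BP_CliffRock is a rock actor that rises vertically when its BridgeUp event fires, apparently as part of a bridge.
; BridgeUp waits DelayTime, then plays the RocksUp timeline.
; Each update lerps Z from the current location toward 6 units above it, so the rise accumulates per tick rather than reaching a fixed target.
; The construction script applies the Mesh variable to the static mesh component.
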(event `BridgeUp`
  (bind (_returnvalue_x _returnvalue_y _returnvalue_z) (`KismetMathLibrary.BreakVector` (`self.K2_GetActorLocation`)))
  (`KismetSystemLibrary.Delay` (`self.DelayTime`))
  (bind (_direction _rocksup) (`Timeline|RocksUp`)
    (:`Update`
      (`self.K2_SetActorLocation` (`KismetMathLibrary.MakeVector` _returnvalue_x _returnvalue_y (`KismetMathLibrary.Lerp` _returnvalue_z (+ _returnvalue_z 6.0) _rocksup))))))

(fn `UserConstructionScript`
  (`StaticMeshComponent.SetStaticMesh` (`self.StaticMesh`) (`self.Mesh`)))