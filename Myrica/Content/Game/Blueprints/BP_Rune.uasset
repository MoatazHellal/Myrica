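; BP_Rune is a rune actor with a floating mesh that can trigger a level sequence when activated.
; A timeline restarts each time it finishes, continuously offsetting the static mesh along X and Z.
; Activate plays the sequence if IsActivable is set; otherwise it sets that flag on every BP_Rune in the level, so a later activation plays it.
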(event `self.ReceiveBeginPlay`
  (bind (_direction _position) (`Timeline|Timeline_0` :!label _label)
    (:`Update`
      (`SceneComponent.K2_SetRelativeLocation` (`self.StaticMesh`) (* _position (10.0 0.0 20.0)) false false))
    (:`Finished`
      (`|ExecutionSequence`
        (:`then_0`
          (goto _label :!via `PlayFromStart`))))))

(event `/Game/Game/BPI_Mechanism.Activate`
  (if (`self.IsActivable`)
    (bind (_outactor _returnvalue) (`LevelSequencePlayer.CreateLevelSequencePlayer` null))
    (`MovieSceneSequencePlayer.Play` _returnvalue)
    (else
      (bind _outactors (`GameplayStatics.GetAllActorsOfClass` "BP_Rune_C"))
      (for _array_element _outactors
        (bind _asbp_rune_04 (cast `/Game/Game/Blueprints/BP_Rune` _array_element))
        (set `/Game/Game/Blueprints/BP_Rune.IsActivable` true _asbp_rune_04)))))

(fn `UserConstructionScript`)