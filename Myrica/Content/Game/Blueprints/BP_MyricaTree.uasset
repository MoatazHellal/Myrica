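; BP_MyricaTree is a tree actor that shows a text prompt nearby and plays the MyricaRevival level sequence when activated.
; Its Sphere reveals the TextRender when an actor whose class is exactly BP_Fey begins overlapping, and hides it when any actor stops overlapping.
; The Activate event creates and plays the sequence player and hides the text, with no guard against repeat activation.
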(event `/Game/Game/BPI_Mechanism.Activate`
  (bind (_outactor _returnvalue) (`LevelSequencePlayer.CreateLevelSequencePlayer` "/Game/Game/Cinematics/MyricaRevival.MyricaRevival"))
  (`MovieSceneSequencePlayer.Play` _returnvalue)
  (`SceneComponent.SetVisibility` (`self.TextRender`) false false))

(event `self.Sphere.OnComponentBeginOverlap`
  (params (OverlappedComponent :type "PrimitiveComponent Object Reference") (OtherActor :type "Actor Object Reference") (OtherComp :type "PrimitiveComponent Object Reference") (OtherBodyIndex :type Integer) (bFromSweep :type Boolean) (SweepResult :type "HitResult Structure (by ref)"))
  (if (== (`GameplayStatics.GetObjectClass` OtherActor) "/Game/Fey/BP_Fey.BP_Fey_C")
    (`SceneComponent.SetVisibility` (`self.TextRender`) true false)))

(event `self.Sphere.OnComponentEndOverlap`
  (params (OverlappedComponent :type "PrimitiveComponent Object Reference") (OtherActor :type "Actor Object Reference") (OtherComp :type "PrimitiveComponent Object Reference") (OtherBodyIndex :type Integer))
  (`SceneComponent.SetVisibility` (`self.TextRender`) false false))

(fn `UserConstructionScript`)