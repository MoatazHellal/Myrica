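; BP_Elevator is an elevator actor that shuttles endlessly between its spawn point and a point a fixed height straight above it.
; BeginPlay caches both endpoints and plays the UpDown timeline, whose Elevation track drives a vector lerp that sets the actor's location without sweeping.
; Each time the timeline finishes, a short delay leads into a FlipFlop that alternates Reverse and Play, so it runs without any trigger.
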(event `self.ReceiveBeginPlay`
  (bind _returnvalue (`self.K2_GetActorLocation`))
  (set `self.StartPosition` _returnvalue)
  (set `self.EndPosition` (+ _returnvalue (0.0 0.0 5000.0)))
  (bind (_direction _elevation) (`Timeline|UpDown` :!label _label)
    (:`Update`
      (`self.K2_SetActorLocation` (`KismetMathLibrary.VLerp` (`self.StartPosition`) (`self.EndPosition`) _elevation)))
    (:`Finished`
      (`KismetSystemLibrary.Delay` 1.0)
      (`/Engine/EditorBlueprintResources/StandardMacros.FlipFlop`
        (:`A`
          (goto _label :!via `Reverse`))
        (:`B`
          (goto _label))))))

(fn `UserConstructionScript`)