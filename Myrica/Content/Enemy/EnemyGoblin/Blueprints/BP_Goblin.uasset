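; Goblin enemy Blueprint that provides a short-range melee attack and a death sequence.
; Attack passes through a DoOnce, then sphere-traces forward for Pawns, playing an attack montage on a hit and killing the target if it is BP_Fey.
; EnemyDie plays the lose montage, unpossesses the AI controller and destroys the goblin after a short delay.
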(event `EnemyDie`
  (`self.PlayAnimMontage` "/Game/Enemy/EnemyGoblin/Animations/Anim_Lose_Montage.Anim_Lose_Montage")
  (`Controller.UnPossess` (`AIBlueprintHelperLibrary.GetAIController` self))
  (`KismetSystemLibrary.Delay` 2.0)
  (`self.K2_DestroyActor`))

(fn `Attack`
  (bind _returnvalue (`self.K2_GetActorLocation`))
  (`/Engine/EditorBlueprintResources/StandardMacros.DoOnce` false
    (:`Completed`
      (bind (_outhit _returnvalue_2) (`KismetSystemLibrary.SphereTraceSingleForObjects` _returnvalue (+ _returnvalue (* (`KismetMathLibrary.GetForwardVector` (`self.K2_GetActorRotation`)) 200.0)) 0.0 (`|MakeArray` "ObjectTypeQuery3" :!type "EObjectTypeQuery Enum")))
      (if _returnvalue_2
        (`self.PlayAnimMontage` "/Game/Enemy/EnemyGoblin/Animations/Anim_Attack1_Montage.Anim_Attack1_Montage")
        (bind _asbp_fey (cast `/Game/Fey/BP_Fey` (`.HitActor` (`GameplayStatics.BreakHitResult` _outhit))))
        (`/Game/Fey/BP_Fey.Die` _asbp_fey)))))

(fn `UserConstructionScript`)